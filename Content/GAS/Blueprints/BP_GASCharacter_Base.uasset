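; Base Gameplay Ability System character with sword melee combat, granted melee and health-regeneration abilities on BeginPlay.
; Sword overlaps with enemy characters send a deal-damage gameplay event to itself with the victim as target, and a helper toggles that collider.
; Ability activation is gated on being alive.
; Death plays a montage and starts a timer of its length, while attribute-change handlers just call their parents.
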(event `self.ReceiveBeginPlay`
  (`parent.ReceiveBeginPlay`)
  (`self.AcquireAbility` (`|MakeArray` "/Game/GAS/Blueprints/Abilities/Melee/GA_Melee.GA_Melee_C" "/Game/GAS/Blueprints/Abilities/HealthRegen/GA_HealthRegen.GA_HealthRegen_C" :!type "GameplayAbility Class Reference")))

(event `self.ReceiveTick`
  (params (DeltaSeconds :type "Float (single-precision)"))
  (`parent.ReceiveTick` DeltaSeconds))

(event `self.SwordCollider.OnComponentBeginOverlap`
  (params (OverlappedComponent :type "PrimitiveComponent Object Reference") (OtherActor :type "Actor Object Reference") (OtherComp :type "PrimitiveComponent Object Reference") (OtherBodyIndex :type Integer) (bFromSweep :type Boolean) (SweepResult :type "HitResult Structure (by ref)"))
  (if (!= OtherActor self)
    (bind _asbp_gascharacter_base (cast `/Game/GAS/Blueprints/BP_GASCharacter_Base` OtherActor))
    (if (`self.IsEnemyCharacter` _asbp_gascharacter_base)
      (`AbilitySystemBlueprintLibrary.SendGameplayEventToActor` self (struct :`TagName` "Ability.Melee.DealDamage") (make `GameplayEventData` (struct) null _asbp_gascharacter_base)))))

(fn `DieCharacter`
  (`parent.DieCharacter`)
  (bind _returnvalue (`self.PlayAnimMontage` "/Game/GAS/Animations/GASCharacter/AM_GASCharacter_Death.AM_GASCharacter_Death"))
  (`KismetSystemLibrary.K2_SetTimerDelegate` (`|CreateDelegate` :!event `K2_DestroyActor`) _returnvalue))

(fn `OnHealthChanged`
  (params (NewPercentage :type "Float (double-precision)"))
  (`parent.OnHealthChanged` NewPercentage))

(fn `OnManaChanged`
  (params (NewPercentage :type "Float (double-precision)"))
  (`parent.OnManaChanged` NewPercentage))

(fn `OnStrengthChanged`
  (params (NewPercentage :type "Float (double-precision)"))
  (`parent.OnStrengthChanged` NewPercentage))

(fn `SetSwordCollision`
  (params (NewType :type "ECollisionEnabled Enum" :default "NoCollision"))
  (bind _swordcollider (`self.SwordCollider`)
    (:`then`
      (`PrimitiveComponent.SetCollisionEnabled` _swordcollider (`local.NewType`)))
    (:`else`)))

(fn `TryActivateAbility`
  (params (InAbilityToActivate :type "GameplayAbility Class Reference"))
  (returns (bSuccess :type Boolean))
  (locals (rValue :type Boolean))
  (`|ExecutionSequence`
    (:`then_0`
      (if (`self.IsAlive`)
        (bind _abilitysystemcomponent (`self.AbilitySystemComponent`)
          (:`then`
            (bind _returnvalue (`AbilitySystemComponent.TryActivateAbilityByClass` _abilitysystemcomponent (`local.InAbilityToActivate`) true))
            (set `local.rValue` _returnvalue))
          (:`else`))))
    (:`then_1`
      (return (`local.rValue`)))))

(fn `UserConstructionScript`)