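; Character Blueprint that uses the Gameplay Ability System to perform a sword melee attack.
; It acquires GA_Melee on BeginPlay, and the MeleeAttack event activates that ability by class.
; Sword collider overlaps with other BP_GASCharacters send an Ability.Melee.DealDamage gameplay event to itself, with the hit character as payload target.
; SetSwordCollision switches the collider's collision mode; a health debug print is left unconnected.
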(event `self.ReceiveBeginPlay`
  (`parent.ReceiveBeginPlay`)
  (`self.AcquireAbility` "/Game/GAS/Blueprints/Abilities/GA_Melee.GA_Melee_C"))

(event `self.ReceiveTick`
  (params (DeltaSeconds :type "Float (single-precision)"))
  (`parent.ReceiveTick` DeltaSeconds))

(event `MeleeAttack`
  (`AbilitySystemComponent.TryActivateAbilityByClass` (`self.AbilitySystemComponent`) "/Game/GAS/Blueprints/Abilities/GA_Melee.GA_Melee_C" true))

(event `self.SwordCollider.OnComponentBeginOverlap`
  (params (OverlappedComponent :type "PrimitiveComponent Object Reference") (OtherActor :type "Actor Object Reference") (OtherComp :type "PrimitiveComponent Object Reference") (OtherBodyIndex :type Integer) (bFromSweep :type Boolean) (SweepResult :type "HitResult Structure (by ref)"))
  (if (!= OtherActor self)
    (bind _asbp_gascharacter (cast `/Game/GAS/Blueprints/BP_GASCharacter` OtherActor))
    (`AbilitySystemBlueprintLibrary.SendGameplayEventToActor` self (struct :`TagName` "Ability.Melee.DealDamage") (make `GameplayEventData` (struct) null _asbp_gascharacter))))

(fn `SetSwordCollision`
  (params (NewType :type "ECollisionEnabled Enum" :default "NoCollision"))
  (bind _swordcollider (`self.SwordCollider`)
    (:`then`
      (`PrimitiveComponent.SetCollisionEnabled` _swordcollider (`local.NewType`)))
    (:`else`)))

(fn `UserConstructionScript`)