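; Player character Blueprint for a Gameplay Ability System setup that mirrors its health, mana and strength on the HUD.
; BeginPlay caches the GAS player controller.
; Overridden attribute-change handlers call their parent, then push the new percentage to the abilities bar widget.
; A shared validity-checking macro resolves that widget through the controller's primary widget, with debug prints when it is missing.
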(event `self.ReceiveBeginPlay`
  (`parent.ReceiveBeginPlay`)
  (bind _asbp_gasplayer_controller (cast `/Game/GAS/Blueprints/BP_GASPlayerController` (`self.GetController`)))
  (set `self.GasPlayerController` _asbp_gasplayer_controller))

(fn `OnHealthChanged`
  (params (NewPercentage :type "Float (double-precision)"))
  (`parent.OnHealthChanged` NewPercentage)
  (bind _wbp_abilitiesbar (`self.GetAbilitiesBarWidget`)
    (:`IsValid`
      (`/Game/GAS/UI/WBP_AbilitiesBar.SetHealth` _wbp_abilitiesbar (`local.NewPercentage`)))
    (:`IsNotValid`
      (`KismetSystemLibrary.PrintString` "BP_GASCharacter_Player: OnHealthChanged" true true (struct :`R` 1.0 :`G` 0.001649 :`A` 1.0)))))

(fn `OnManaChanged`
  (params (NewPercentage :type "Float (double-precision)"))
  (`parent.OnManaChanged` NewPercentage)
  (bind _wbp_abilitiesbar (`self.GetAbilitiesBarWidget`)
    (:`IsValid`
      (`/Game/GAS/UI/WBP_AbilitiesBar.SetMana` _wbp_abilitiesbar (`local.NewPercentage`)))
    (:`IsNotValid`
      (`KismetSystemLibrary.PrintString` "BP_GASCharacter_Player: OnManaChanged" true true (struct :`R` 1.0 :`G` 0.001649 :`A` 1.0)))))

(fn `OnStrengthChanged`
  (params (NewPercentage :type "Float (double-precision)"))
  (`parent.OnStrengthChanged` NewPercentage)
  (bind _wbp_abilitiesbar (`self.GetAbilitiesBarWidget`)
    (:`IsValid`
      (`/Game/GAS/UI/WBP_AbilitiesBar.SetStrength` _wbp_abilitiesbar (`local.NewPercentage`)))
    (:`IsNotValid`
      (`KismetSystemLibrary.PrintString` "BP_GASCharacter_Player: OnStrengthChanged" true true (struct :`R` 1.0 :`G` 0.001649 :`A` 1.0)))))

(fn `UserConstructionScript`
  (`parent.UserConstructionScript`))