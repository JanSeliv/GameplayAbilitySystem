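; GA_Dash is a Gameplay Ability that makes the owning character dash forward while damaging and stunning targets it hits.
; On activation it commits, plays a montage, and pushes the owner with an impulse lasting the montage length.
; It waits for a dash damage gameplay event, then pushes and stuns the event's target character and applies the dash damage effect.
; A failed commit or invalid owner only prints a failure message.
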(event `self.K2_ActivateAbility`
  (`parent.K2_ActivateAbility`)
  (bind _bsuccesscommit (`self.CommitAndPlayMontage`))
  (if _bsuccesscommit
    (bind _owningcharacter (`self.OwningCharacter`)
      (:`then`
        (`/Game/GAS/Blueprints/BP_GASCharacter_Base.PushMe` _owningcharacter (`/Game/GAS/Blueprints/BP_GASCharacter_Base.GetImpulse` _owningcharacter 2000.0) (`self.MontageLength`) false true)
        (bind (_asynctaskproxy _payload) (`AbilityTask_WaitGameplayEvent.WaitGameplayEvent` (struct :`TagName` "Ability.Dash.DamageEvent") null)
          (:`EventReceived`
            (bind _asbp_gascharacter_base (cast `/Game/GAS/Blueprints/BP_GASCharacter_Base` (`.Target` (break `GameplayEventData` _payload))))
            (`/Game/GAS/Blueprints/BP_GASCharacter_Base.PushMe` _asbp_gascharacter_base (`/Game/GAS/Blueprints/BP_GASCharacter_Base.GetImpulse` (`self.OwningCharacter`) 2000.0) (`self.MontageLength`) true false)
            (`self.Apply Effect to Target` (`.Target` (break `GameplayEventData` _payload)) "/Game/GAS/Blueprints/Abilities/Dash/GE_Dash_Damage.GE_Dash_Damage_C"))))
      (:`else`
        (`KismetSystemLibrary.PrintString` "GA_Dash: Dash: FAIL" true true (struct :`R` 1.0 :`G` 0.004012 :`A` 1.0) :!label _label)))
    (else
      (goto _label))))

(event `self.K2_OnEndAbility`
  (params (bWasCancelled :type Boolean))
  (`parent.K2_OnEndAbility` bWasCancelled))