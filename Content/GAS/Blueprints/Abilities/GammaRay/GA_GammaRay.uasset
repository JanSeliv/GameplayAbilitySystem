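; Gameplay ability for a Gamma Ray attack that, once committed and after a short montage delay, attaches a ray actor to a socket on the character mesh and enables camera-controlled rotation.
; Gameplay damage events then apply a damage effect and a stunning forward impulse to the target, briefly toggling overlap-only-once on the owner, or end the ability when cost is insufficient.
; Ending restores rotation, destroys the ray and stops the montage.
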(event `self.K2_ActivateAbility`
  (`parent.K2_ActivateAbility`)
  (bind _bsuccesscommit (`self.CommitAbilityBase` false))
  (if _bsuccesscommit
    (`KismetSystemLibrary.Delay` 0.3) ; montage time\n@todo spawn on event
    (`|ExecutionSequence`
      (:`then_0`
        (bind _owninggascharacter (`self.OwningGASCharacter`)
          (:`then`
            (`GASCharacter.SetCameraControlRotation` _owninggascharacter true)
            (bind _mesh (`Character.Mesh` (`self.OwningGASCharacter`))
              (:`then`
                (if (`SceneComponent.DoesSocketExist` _mesh (`self.SocketToAttach`))
                  (bind (_asynctaskproxy _spawnedactor) (`AbilityTask_SpawnActor.SpawnActor` (struct) "/Game/GAS/Blueprints/Abilities/GammaRay/BP_GammaRay.BP_GammaRay_C" (`self.OwningGASCharacter`))
                    (:`Success`
                      (bind _output_get (set `self.GammaRayActor` _spawnedactor))
                      (`Actor.K2_AttachToComponent` _output_get _mesh (`self.SocketToAttach`) "SnapToTarget" "SnapToTarget" "KeepRelative" true)))))
              (:`else`)))
          (:`else`)))
      (:`then_1`
        (bind (_asynctaskproxy_2 _payload) (`AbilityTask_WaitGameplayEvent.WaitGameplayEvent` (struct :`TagName` "Ability.GammaRay.DamageEvent") null)
          (:`EventReceived`
            (if (`self.IsCostEnough`)
              (bind _asgascharacter (cast `GASCharacter` (`.Target` (break `GameplayEventData` _payload))))
              (`|ExecutionSequence`
                (:`then_0`
                  (`self.BP_ApplyGameplayEffectToTarget` (`AbilitySystemBlueprintLibrary.AbilityTargetDataFromActor` _asgascharacter) "/Game/GAS/Blueprints/Abilities/GammaRay/GE_GammaRay_Damage.GE_GammaRay_Damage_C"))
                (:`then_1`
                  (bind _owninggascharacter_2 (`self.OwningGASCharacter`)
                    (:`then`
                      (`GASCharacter.SetOverlapOnlyOnce` _owninggascharacter_2 true)
                      (`GASCharacter.AddImpulse` _asgascharacter (`/Game/GAS/Blueprints/BP_GASCharacter_Base.GetForwardImpulse` _owninggascharacter_2 400.0) 0.05 true false))
                    (:`else`)))
                (:`then_2`
                  (`KismetSystemLibrary.Delay` 1.0)
                  (bind _owninggascharacter_3 (`self.OwningGASCharacter`)
                    (:`then`
                      (`GASCharacter.SetOverlapOnlyOnce` _owninggascharacter_3 false))
                    (:`else`))))
              (else
                (`self.K2_EndAbility`)))))))))

(event `self.K2_OnEndAbility`
  (params (bWasCancelled :type Boolean))
  (`parent.K2_OnEndAbility` bWasCancelled)
  (`|ExecutionSequence`
    (:`then_0`
      (bind _owninggascharacter (`self.OwningGASCharacter`)
        (:`then`
          (`GASCharacter.SetCameraControlRotation` _owninggascharacter false))
        (:`else`)))
    (:`then_1`
      (bind _gammarayactor (`self.GammaRayActor`)
        (:`then`
          (`Actor.K2_DestroyActor` _gammarayactor))
        (:`else`)))
    (:`then_2`
      (bind _owninggascharacter_2 (`self.OwningGASCharacter`)
        (:`then`
          (`Character.StopAnimMontage` _owninggascharacter_2 (`self.AnimMontage`)))
        (:`else`)))))