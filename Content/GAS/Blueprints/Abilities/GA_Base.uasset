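; GA_Base is a gameplay ability base that manages montage playback and sword collision for character attacks.
; CommitMontageEnd commits the ability on the owning Character and, on success, enables sword collision, plays the montage and starts a one-shot timer for its duration, returning the commit result.
; Ending the ability disables sword collision.
; Collision changes always target player 0's BP_GASCharacter rather than the ability's owner.
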(event `self.K2_ActivateAbility`
  (`parent.K2_ActivateAbility`))

(event `self.K2_OnEndAbility`
  (params (bWasCancelled :type Boolean))
  (`parent.K2_OnEndAbility` bWasCancelled)
  (`self.SetSwordCollision` "NoCollision"))

(fn `CommitMontageEnd`
  (params (AnimMontage :type "AnimMontage Object Reference"))
  (returns (bSuccessCommit :type Boolean))
  (locals (rValue :type Boolean :default false) (OwnerCharacter :type "Character Object Reference"))
  (`|ExecutionSequence`
    (:`then_0`
      (`local.AnimMontage`
        (:`then`
          (bind _ascharacter (cast `Character` (`self.GetOwningActorFromActorInfo`)))
          (set `local.OwnerCharacter` _ascharacter)
          (bind _returnvalue (`self.K2_CommitAbility`))
          (set `local.rValue` _returnvalue))
        (:`else`)))
    (:`then_1`
      (if (`local.rValue`)
        (`self.SetSwordCollision` "QueryAndPhysics")
        (bind _returnvalue_2 (`Character.PlayAnimMontage` (`local.OwnerCharacter`) (`local.AnimMontage`) 1.0 "None"))
        (`KismetSystemLibrary.K2_SetTimerDelegate` (`|CreateDelegate` :!event `K2_EndAbility`) _returnvalue_2)))
    (:`then_2`
      (return (`local.rValue`)))))

(fn `SetSwordCollision`
  (params (NewType :type "ECollisionEnabled Enum" :default "NoCollision"))
  (bind _asbp_gascharacter (cast `/Game/GAS/Blueprints/BP_GASCharacter` (`GameplayStatics.GetPlayerCharacter` 0)))
  (`/Game/GAS/Blueprints/BP_GASCharacter.SetSwordCollision` _asbp_gascharacter (`local.NewType`)))