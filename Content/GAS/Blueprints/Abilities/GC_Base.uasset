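; Base gameplay cue that plays a particle effect on its target when executed.
; OnExecute spawns the ParticleSystem variable attached to the target's root component, snapped to it, if that component is valid.
; It returns true only if both the parent OnExecute succeeds and a valid emitter was spawned.
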(fn `OnExecute`
  (params (MyTarget :type "Actor Object Reference") (Parameters :type "GameplayCueParameters Structure (by ref)"))
  (returns (ReturnValue :type Boolean))
  (locals (rValue :type Boolean))
  (`|ExecutionSequence`
    (:`then_0`
      (bind _rootcomponent (`Actor.RootComponent` (`local.MyTarget`))
        (:`then`
          (bind _returnvalue (`GameplayStatics.SpawnEmitterAttached` (`self.ParticleSystem`) _rootcomponent "None" (0.0 0.0 0.0) (struct) (1.0 1.0 1.0) "SnapToTarget"))
          (set `local.rValue` (`KismetSystemLibrary.IsValid` _returnvalue)))
        (:`else`)))
    (:`then_1`
      (return (and (`parent.OnExecute` MyTarget Parameters) (`local.rValue`))))))