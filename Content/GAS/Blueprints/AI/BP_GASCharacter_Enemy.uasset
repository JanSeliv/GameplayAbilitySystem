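; Enemy character Blueprint for the GAS-based AI, which keeps its health bar widget in sync with its health.
; A health-change handler receives the new percentage and, if the HealthBarWidget component is valid, casts its user widget to WBP_HealthBar to update it.
; The event graph holds only disabled stub events, and the construction script just calls the parent.
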(fn `OnHealthChange_0`
  (params (NewPercentage :type "Float (double-precision)" :default 0.0))
  (bind _healthbarwidget (`self.HealthBarWidget`)
    (:`then`
      (bind _aswbp_health_bar (cast `/Game/GAS/UI/WBP_HealthBar` (`WidgetComponent.GetUserWidgetObject` _healthbarwidget)))
      (`/Game/GAS/UI/WBP_HealthBar.SetPercentage` _aswbp_health_bar (`local.NewPercentage`)))
    (:`else`)))

(fn `UserConstructionScript`
  (`parent.UserConstructionScript`))