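; Behavior tree task that gives a GAS enemy the first player's character as its target.
; While the enemy is alive, it keeps any Character already stored under the literal "Target" blackboard name, otherwise writes the player to the TargetKey selector.
; It then finishes with a result flag that is set true only when a target is kept or assigned.
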(fn `ReceiveExecuteAI`
  (params (OwnerController :type "AIController Object Reference") (ControlledPawn :type "Pawn Object Reference"))
  (locals (rValue :type Boolean))
  (`parent.ReceiveExecuteAI` OwnerController ControlledPawn)
  (`|ExecutionSequence`
    (:`then_0`
      (bind _asbp_gascharacter_enemy (cast `/Game/GAS/Blueprints/AI/BP_GASCharacter_Enemy` (`local.ControlledPawn`)))
      (if (`GASCharacter.IsAlive` _asbp_gascharacter_enemy)
        (cast `Character` (`BlackboardComponent.GetValueAsObject` (`BTFunctionLibrary.GetOwnersBlackboard`) "Target")
          (:`then`
            _)
          (:`CastFailed`
            (bind _asgascharacter (cast `GASCharacter` (`GameplayStatics.GetPlayerCharacter` 0)))
            (`BTFunctionLibrary.SetBlackboardValueAsObject` (`self.TargetKey`) _asgascharacter)))
        (set `local.rValue` true)))
    (:`then_1`
      (`self.FinishExecute` (`local.rValue`)))))