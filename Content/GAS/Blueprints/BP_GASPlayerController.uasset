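; Player controller for the GAS project that builds the HUD and turns input into gameplay ability activations on the player character.
; BeginPlay creates the primary widget, keeps its abilities bar and caches the controlled GAS character.
; The primary action triggers the melee ability, while numbered ability presses activate whatever class sits in the matching bar slot.
; Overridden AddAbilityToUI places new abilities in the bar's next free slot.
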(event `self.ReceiveBeginPlay`
  (`parent.ReceiveBeginPlay`)
  (`|ExecutionSequence`
    (:`then_0`
      (bind _returnvalue (`|CreateWidget` "/Game/GAS/UI/WBP_Primary.WBP_Primary_C"))
      (set `self.AbilitiesBarWidget` (`/Game/GAS/UI/WBP_Primary.WBP_AbilitiesBar` _returnvalue))
      (`UserWidget.AddToViewport` _returnvalue 0)
      (`WidgetBlueprintLibrary.SetFocusToGameViewport`))
    (:`then_1`
      (bind _asbp_gascharacter_player (cast `/Game/GAS/Blueprints/BP_GASCharacter_Player` (`self.K2_GetPawn`)))
      (set `self.ControlledGasPlayer` _asbp_gascharacter_player))))

(event `self.ReceiveTick`
  (params (DeltaSeconds :type "Float (single-precision)"))
  (`parent.ReceiveTick` DeltaSeconds))

(event `InputAction|PrimaryAction`
  (params (Key :type "Key Structure"))
  (:`Pressed`
    (bind _controlledgasplayer (`self.ControlledGasPlayer`)
      (:`then`
        (`GASCharacter.TryActivateAbility` _controlledgasplayer "/Game/GAS/Blueprints/Abilities/Melee/GA_Melee.GA_Melee_C"))
      (:`else`))))

(fn `AddAbilityToUI`
  (params (InAbilityBaseClass :type "GameplayAbilityBase Class Reference"))
  (`parent.AddAbilityToUI` InAbilityBaseClass)
  (bind _abilitiesbarwidget (`self.AbilitiesBarWidget`)
    (:`then`
      (`/Game/GAS/UI/WBP_AbilitiesBar.AddAbilityToUI` _abilitiesbarwidget (`/Game/GAS/UI/WBP_AbilitiesBar.GetFreeSlotIndex` _abilitiesbarwidget) (`local.InAbilityBaseClass`)))
    (:`else`)))

(fn `OnAbilityPressed`
  (params (AbilityN :type Integer))
  (`parent.OnAbilityPressed` AbilityN)
  (bind _abilitiesbarwidget (`self.AbilitiesBarWidget`)
    (:`then`
      (`self.ControlledGasPlayer`
        (:`then`
          (bind _abilityclass (`/Game/GAS/UI/WBP_AbilitySlot.AbilityClass` (`/Game/GAS/UI/WBP_AbilitiesBar.GetSlotWidgetByIndex` _abilitiesbarwidget (- (`local.AbilityN`) 1)))
            (:`then`
              (`GASCharacter.TryActivateAbility` (`self.ControlledGasPlayer`) _abilityclass))
            (:`else`)))
        (:`else`)))
    (:`else`)))

(fn `UserConstructionScript`)